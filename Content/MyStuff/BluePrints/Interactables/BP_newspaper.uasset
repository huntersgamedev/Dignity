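; BP_newspaper is an interactable newspaper that shows dialogue options and can unlock an option on a linked pay phone.
; Interact passes its text, replies and button states to the interact HUD widget, cached after a BeginPlay delay, then switches input to UI-only with the cursor shown.
; Trigger makes the third button in the PayPhone's InteractStatus visible, then looks up the HUD again to set the interact reply.
; A fail-reply assignment is present but unconnected.
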(event `self.ReceiveBeginPlay`
  (`KismetSystemLibrary.Delay` 2.0)
  (bind _foundwidgets (`WidgetBlueprintLibrary.GetAllWidgetsOfClass` "/Game/MyStuff/UI/WID_interactHUD.WID_interactHUD_C" false))
  (set `self.InteractHUD` (`|GetArrayItem` _foundwidgets)))

(event `/Game/MyStuff/BluePrints/InteractSystem/Interactable.Interact`
  (bind _returnvalue (`GameplayStatics.GetPlayerController` 0))
  (`/Game/MyStuff/UI/WID_interactHUD.SetOptionVisibility` (`self.InteractHUD`) (`self.InteractText`) (`self.InteractReply`) self (`self.InteractStatus`))
  (`UserWidget.AddToViewport` (`self.InteractHUD`) 0)
  (set `PlayerController.bShowMouseCursor` true _returnvalue)
  (`WidgetBlueprintLibrary.SetInputMode_UIOnlyEx` _returnvalue (`self.InteractHUD`)))

(event `/Game/MyStuff/BluePrints/InteractSystem/Interactable.Trigger`
  (params (Option :type Integer))
  (bind _interactstatus (`/Game/MyStuff/BluePrints/Interactables/BP_PayPhone.InteractStatus` (`self.PayPhone`)))
  (bind ((`Text_4_0927B8D549F63D4858D81F93306A8426` _text) (`type_7_4742D12F42B0E80D58A507BFD547AEA1` _type)) (break `/Game/MyStuff/BluePrints/InteractSystem/STR_ButtonStatus` (`|GetArrayItem` _interactstatus 2)))
  (`KismetArrayLibrary.Array_Set` _interactstatus 2 (make `/Game/MyStuff/BluePrints/InteractSystem/STR_ButtonStatus` true _text _type))
  (bind _foundwidgets (`WidgetBlueprintLibrary.GetAllWidgetsOfClass` "/Game/MyStuff/UI/WID_interactHUD.WID_interactHUD_C" false))
  (`/Game/MyStuff/UI/WID_interactHUD.SetInteractReply` (`|GetArrayItem` _foundwidgets)))

(fn `UserConstructionScript`)