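; BP_Barista is an interactable barista that sells to the player through dialogue options in the shared WID_interactHUD.
; Interact feeds its text, replies and button states to the widget, then switches to UI-only input with a cursor.
; Trigger charges the player a fixed price and shows the reply, or a failure reply if money is short.
; Buying option 2 also makes a key code option visible on the linked KeyDoor.
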(event `self.ReceiveBeginPlay`
  (`KismetSystemLibrary.Delay` 2.0)
  (bind _foundwidgets (`WidgetBlueprintLibrary.GetAllWidgetsOfClass` "/Game/MyStuff/UI/WID_interactHUD.WID_interactHUD_C" false))
  (set `self.InteractHUD` (`|GetArrayItem` _foundwidgets)))

(event `/Game/MyStuff/BluePrints/InteractSystem/Interactable.Interact`
  (bind _returnvalue (`GameplayStatics.GetPlayerController` 0))
  (`/Game/MyStuff/UI/WID_interactHUD.SetOptionVisibility` (`self.InteractHUD`) (`self.InteractText`) (`self.InteractReply`) self (`self.InteractStatus`))
  (`UserWidget.AddToViewport` (`self.InteractHUD`) 0)
  (set `PlayerController.bShowMouseCursor` true _returnvalue)
  (`WidgetBlueprintLibrary.SetInputMode_UIOnlyEx` _returnvalue (`self.InteractHUD`)))

(event `/Game/MyStuff/BluePrints/InteractSystem/Interactable.Trigger`
  (params (Option :type Integer))
  (bind _asfirst_person_character (cast `/Game/FirstPersonBP/Blueprints/FirstPersonCharacter` (`GameplayStatics.GetPlayerCharacter` 0) :!pure true))
  (if (>= (`/Game/FirstPersonBP/Blueprints/FirstPersonCharacter.Total Money` _asfirst_person_character) 2.75)
    (if (== Option 2)
      (`self.GiveKeyCode`))
    (`/Game/FirstPersonBP/Blueprints/FirstPersonCharacter.TakeMoney` _asfirst_person_character 2.75)
    (bind _foundwidgets (`WidgetBlueprintLibrary.GetAllWidgetsOfClass` "/Game/MyStuff/UI/WID_interactHUD.WID_interactHUD_C" false))
    (`/Game/MyStuff/UI/WID_interactHUD.SetInteractReply` (`|GetArrayItem` _foundwidgets))
    (else
      (bind _foundwidgets_2 (`WidgetBlueprintLibrary.GetAllWidgetsOfClass` "/Game/MyStuff/UI/WID_interactHUD.WID_interactHUD_C" false))
      (set `/Game/MyStuff/UI/WID_interactHUD.InteractText` (`self.InteractFailReply`) (`|GetArrayItem` _foundwidgets_2)))))

(fn `GiveKeyCode`
  (bind _interactstatus (`/Game/MyStuff/BluePrints/Interactables/BP_KEYDoor.InteractStatus` (`self.KeyDoor`)))
  (bind (_visible_ _text _type) (break `/Game/MyStuff/BluePrints/InteractSystem/STR_ButtonStatus` (`|GetArrayItem` _interactstatus 2)))
  (`KismetArrayLibrary.Array_Set` _interactstatus 2 (make `/Game/MyStuff/BluePrints/InteractSystem/STR_ButtonStatus` true _text _type)))

(fn `UserConstructionScript`)