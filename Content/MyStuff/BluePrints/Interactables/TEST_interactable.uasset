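; Test interactable actor that opens the interaction HUD when the player interacts with it.
; Interact finds the existing WID_interactHUD widget, passes it the prompt text, reply, button status and itself, then adds it to the viewport.
; It shows the mouse cursor and switches to UI-only input focused on that widget.
; A Trigger event only prints a debug string.
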(event `/Game/MyStuff/BluePrints/InteractSystem/Interactable.Interact`
  (bind _returnvalue (`GameplayStatics.GetPlayerController` 0))
  (bind _foundwidgets (`WidgetBlueprintLibrary.GetAllWidgetsOfClass` "/Game/MyStuff/UI/WID_interactHUD.WID_interactHUD_C" false))
  (bind _output (`|GetArrayItem` _foundwidgets))
  (`/Game/MyStuff/UI/WID_interactHUD.SetOptionVisibility` _output (`self.InteractText`) (`self.InteractReply`) self (`self.InteractStatus`))
  (`UserWidget.AddToViewport` _output 0)
  (set `PlayerController.bShowMouseCursor` true _returnvalue)
  (`WidgetBlueprintLibrary.SetInputMode_UIOnlyEx` _returnvalue _output))

(event `/Game/MyStuff/BluePrints/InteractSystem/Interactable.Trigger`
  (params (Option :type Integer))
  (`KismetSystemLibrary.PrintString` "triggerbutton"))

(fn `UserConstructionScript`)