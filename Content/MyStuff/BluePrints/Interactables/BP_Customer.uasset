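; BP_Customer is an interactable customer actor that opens the interaction HUD when the player interacts with it.
; On BeginPlay it waits briefly, then caches the first existing WID_interactHUD widget, with the delay working around a misfire.
; Interact passes its text, reply, status and itself to that widget, adds it to the viewport, shows the cursor and switches input to UI only.
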(event `self.ReceiveBeginPlay`
  ;[1 1 1] Gets a reference to the interact HUD there is a delay because it miss fires if there is not
  (`KismetSystemLibrary.Delay` 2.0)
  (bind _foundwidgets (`WidgetBlueprintLibrary.GetAllWidgetsOfClass` "/Game/MyStuff/UI/WID_interactHUD.WID_interactHUD_C" false))
  (set `self.InteractHUD` (`|GetArrayItem` _foundwidgets)))

(event `/Game/MyStuff/BluePrints/InteractSystem/Interactable.Interact`
  (bind _returnvalue (`GameplayStatics.GetPlayerController` 0))
  ;[1 1 1] Sets up and launches interact Hud for the customer
  (`/Game/MyStuff/UI/WID_interactHUD.SetOptionVisibility` (`self.InteractHUD`) (`self.InteractText`) (`self.InteractReply`) self (`self.InteractStatus`))
  (`UserWidget.AddToViewport` (`self.InteractHUD`) 0)
  (set `PlayerController.bShowMouseCursor` true _returnvalue)
  (`WidgetBlueprintLibrary.SetInputMode_UIOnlyEx` _returnvalue (`self.InteractHUD`)))

(fn `UserConstructionScript`)