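; BP_KEYDoor is an interactable door that stays locked until its Trigger event activates it.
; While locked, Interact shows the WID_interactHUD prompt, found shortly after BeginPlay, with cursor and UI-only input.
; Trigger unlocks and toggles the door and updates the HUD reply; later interactions toggle it directly.
; A timeline swings the root 90 degrees in yaw and reverses to close; money-charging nodes are disconnected.
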(event `self.ReceiveBeginPlay`
  (`KismetSystemLibrary.Delay` 2.0)
  (bind _foundwidgets (`WidgetBlueprintLibrary.GetAllWidgetsOfClass` "/Game/MyStuff/UI/WID_interactHUD.WID_interactHUD_C" false))
  (set `self.InteractHUD` (`|GetArrayItem` _foundwidgets))
  (set `self.OrginalRotation` (`SceneComponent.K2_GetComponentRotation` (`self.DefaultSceneRoot`))))

(event `/Game/MyStuff/BluePrints/InteractSystem/Interactable.Interact`
  (bind _returnvalue (`GameplayStatics.GetPlayerController` 0))
  (if (`self.Activated?`)
    (`self.Open/closeDoor`)
    (else
      (`/Game/MyStuff/UI/WID_interactHUD.SetOptionVisibility` (`self.InteractHUD`) (`self.InteractText`) (`self.InteractReply`) self (`self.InteractStatus`))
      (`UserWidget.AddToViewport` (`self.InteractHUD`) 0)
      (set `PlayerController.bShowMouseCursor` true _returnvalue)
      (`WidgetBlueprintLibrary.SetInputMode_UIOnlyEx` _returnvalue (`self.InteractHUD`)))))

(event `/Game/MyStuff/BluePrints/InteractSystem/Interactable.Trigger`
  (params (Option :type Integer))
  (set `self.Activated?` true)
  (`self.Open/closeDoor`)
  (bind _foundwidgets (`WidgetBlueprintLibrary.GetAllWidgetsOfClass` "/Game/MyStuff/UI/WID_interactHUD.WID_interactHUD_C" false))
  (`/Game/MyStuff/UI/WID_interactHUD.SetInteractReply` (`|GetArrayItem` _foundwidgets)))

(event `Open/closeDoor`
  (if (`self.Closed?`)
    (set `self.Closed?` false)
    (bind (_direction _openclose) (`Timeline|OpenCloseDoor` :!label _label)
      (:`Update`
        (`SceneComponent.K2_SetWorldRotation` (`self.DefaultSceneRoot`) (`KismetMathLibrary.RLerp` (`self.OrginalRotation`) (`KismetMathLibrary.MakeRotator` (.roll (`self.OrginalRotation`)) (.pitch (`self.OrginalRotation`)) (+ (.yaw (`self.OrginalRotation`)) 90.0)) _openclose true) false false)))
    (else
      (set `self.Closed?` true)
      (goto _label :!via `Reverse`))))

(fn `UserConstructionScript`)