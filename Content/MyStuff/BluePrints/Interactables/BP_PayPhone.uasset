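; BP_PayPhone is an interactable pay phone that charges the player per call and can summon a car tow.
; Interact opens the shared interact HUD with its options in UI-only input.
; Trigger checks TotalMoney, with a higher threshold once the tow is called, then takes the fee or shows a failure reply.
; The correct option plays the CarTow sequence, destroys MoneyBlock and hides that option.
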(event `self.ReceiveBeginPlay`
  (`KismetSystemLibrary.Delay` 2.0)
  (bind _foundwidgets (`WidgetBlueprintLibrary.GetAllWidgetsOfClass` "/Game/MyStuff/UI/WID_interactHUD.WID_interactHUD_C" false))
  (set `self.InteractHUD` (`|GetArrayItem` _foundwidgets)))

(event `/Game/MyStuff/BluePrints/InteractSystem/Interactable.Interact`
  (bind _returnvalue (`GameplayStatics.GetPlayerController` 0))
  (`/Game/MyStuff/UI/WID_interactHUD.SetOptionVisibility` (`self.InteractHUD`) (`self.InteractText`) (`self.InteractReply`) self (`self.InteractStatus`))
  (`UserWidget.AddToViewport` (`self.InteractHUD`) 0)
  (set `PlayerController.bShowMouseCursor` true _returnvalue)
  (`WidgetBlueprintLibrary.SetInputMode_UIOnlyEx` _returnvalue (`self.InteractHUD`)))

(event `/Game/MyStuff/BluePrints/InteractSystem/Interactable.Trigger`
  (params (Option :type Integer))
  (bind _asfirst_person_character (cast `/Game/FirstPersonBP/Blueprints/FirstPersonCharacter` (`GameplayStatics.GetPlayerCharacter` 0) :!pure true))
  (bind _total_money (`/Game/FirstPersonBP/Blueprints/FirstPersonCharacter.Total Money` _asfirst_person_character))
  (if (`self.TowCalled?`)
    (if (>= _total_money 3.0)
      (`/Game/FirstPersonBP/Blueprints/FirstPersonCharacter.TakeMoney` _asfirst_person_character 0.25 :!label _label)
      (bind _foundwidgets (`WidgetBlueprintLibrary.GetAllWidgetsOfClass` "/Game/MyStuff/UI/WID_interactHUD.WID_interactHUD_C" false))
      (`/Game/MyStuff/UI/WID_interactHUD.SetInteractReply` (`|GetArrayItem` _foundwidgets))
      (else
        (bind _foundwidgets_2 (`WidgetBlueprintLibrary.GetAllWidgetsOfClass` "/Game/MyStuff/UI/WID_interactHUD.WID_interactHUD_C" false :!label _label_2))
        (set `/Game/MyStuff/UI/WID_interactHUD.InteractText` (`self.InteractFailReply`) (`|GetArrayItem` _foundwidgets_2))))
    (elif (>= _total_money 0.25)
      (if (== Option 2)
        (`self.CorrectNumberCalled`)
        (goto _label)
        (else
          (goto _label)))
      (else
        (goto _label_2)))))

(fn `CorrectNumberCalled`
  (bind (_outactor _returnvalue) (`LevelSequencePlayer.CreateLevelSequencePlayer` "/Game/MyStuff/Sequence/CarTow.CarTow" (make `MovieSceneSequencePlaybackSettings` 0 1.0 false 0.0 false false false false false false true)))
  (`MovieSceneSequencePlayer.Play` _returnvalue)
  (`self.K2_DestroyActor` (`self.MoneyBlock`))
  (set `self.TowCalled?` true)
  (`KismetArrayLibrary.Array_Set` (`self.InteractStatus`) 2 (make `/Game/MyStuff/BluePrints/InteractSystem/STR_ButtonStatus` false)))

(fn `UserConstructionScript`)