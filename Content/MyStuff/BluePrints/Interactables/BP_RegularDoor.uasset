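; BP_RegularDoor is an interactable door that swings open and closed when interacted with.
; On BeginPlay it stores the door mesh's world rotation as the original.
; Each interaction flips a Closed flag and plays or reverses a timeline, which lerps the root component's rotation between the original and 90 degrees of added yaw.
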(event `self.ReceiveBeginPlay`
  (set `self.OrginalRotation` (`SceneComponent.K2_GetComponentRotation` (`self.Door`))))

(event `/Game/MyStuff/BluePrints/InteractSystem/Interactable.Interact`
  (`self.Open/closeDoor`))

(event `Open/closeDoor`
  (if (`self.closed?`)
    (set `self.closed?` false)
    (bind (_direction _opendoor) (`Timeline|DoorOpen` :!label _label)
      (:`Update`
        (`SceneComponent.K2_SetWorldRotation` (`self.DefaultSceneRoot`) (`KismetMathLibrary.RLerp` (`self.OrginalRotation`) (`KismetMathLibrary.MakeRotator` (.roll (`self.OrginalRotation`)) (.pitch (`self.OrginalRotation`)) (+ (.yaw (`self.OrginalRotation`)) 90.0)) _opendoor true) false false)))
    (else
      (set `self.closed?` true)
      (goto _label :!via `Reverse`))))

(fn `UserConstructionScript`)