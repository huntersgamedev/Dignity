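; Pedestrian for the begging feature that walks a fixed world-space path and either gives the player change or refuses.
; On BeginPlay it caches the player HUD and runs a timeline lerp between two hardcoded points, destroying itself when finished.
; DropCoinOrnot, not called within this Blueprint, uses a DoOnce and nested random rolls to show a refusal or gift on the HUD, adding small amounts to FirstPersonCharacter's money.
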(event `WalkingPedestrian`
  ;[1 1 1] Handles animating the pedestrian from point A to point B
  (bind (_direction _walking) (`Timeline|Pedestrian`)
    (:`Update`
      (`SceneComponent.K2_SetWorldLocation` (`self.DefaultSceneRoot`) (`KismetMathLibrary.VLerp` (-687.359009 -50.673706 87.965424) (-687.359009 -1356.790283 87.965424) _walking) false false))
    (:`Finished`
      (`self.K2_DestroyActor`))))

(event `self.ReceiveBeginPlay`
  ;[1 1 1] Gets a reference to HUD and starts walking lerp
  (`self.WalkingPedestrian`)
  (bind _foundwidgets (`WidgetBlueprintLibrary.GetAllWidgetsOfClass` "/Game/MyStuff/UI/WID_PlayerHud.WID_PlayerHud_C"))
  (set `self.playerHud` (`|GetArrayItem` _foundwidgets)))

(event `DropCoinOrnot`
  ;[1 1 1] Determines wether this pedestrian will give change when begging
  (`/Engine/EditorBlueprintResources/StandardMacros.DoOnce` false
    (:`Completed`
      (switch `int` (`KismetMathLibrary.RandomIntegerInRange` 0 5)
        (:`0`
          (switch `int` (`KismetMathLibrary.RandomIntegerInRange` 0 5) :!label _label
            (:`0`
              (`/Game/MyStuff/UI/WID_PlayerHud.RefusedBag` (`self.playerHud`)))
            (:`1`
              (`/Game/MyStuff/UI/WID_PlayerHud.GaveMoney` (`self.playerHud`) :!label _label_2)
              (`/Game/FirstPersonBP/Blueprints/FirstPersonCharacter.Add Money` (cast `/Game/FirstPersonBP/Blueprints/FirstPersonCharacter` (`GameplayStatics.GetPlayerCharacter` 0) :!pure true) 0.1))
            (:`2`
              (`/Game/MyStuff/UI/WID_PlayerHud.GaveMoney` (`self.playerHud`) :!label _label_3)
              (`/Game/FirstPersonBP/Blueprints/FirstPersonCharacter.Add Money` (cast `/Game/FirstPersonBP/Blueprints/FirstPersonCharacter` (`GameplayStatics.GetPlayerCharacter` 0) :!pure true) 0.05))
            (:`3`
              (goto _label_2))
            (:`4`
              (goto _label_3))
            (:`5`
              (goto _label_3))))
        (:`1`
          (goto _label))
        (:`2`
          (goto _label))
        (:`3`
          (switch `int` (`KismetMathLibrary.RandomIntegerInRange` 0 5) :!label _label_4
            (:`0`
              (`/Game/MyStuff/UI/WID_PlayerHud.GaveMoney` (`self.playerHud`) :!label _label_5)
              (`/Game/FirstPersonBP/Blueprints/FirstPersonCharacter.Add Money` (cast `/Game/FirstPersonBP/Blueprints/FirstPersonCharacter` (`GameplayStatics.GetPlayerCharacter` 0) :!pure true) 0.1))
            (:`1`
              (`/Game/MyStuff/UI/WID_PlayerHud.GaveMoney` (`self.playerHud`) :!label _label_6)
              (`/Game/FirstPersonBP/Blueprints/FirstPersonCharacter.Add Money` (cast `/Game/FirstPersonBP/Blueprints/FirstPersonCharacter` (`GameplayStatics.GetPlayerCharacter` 0) :!pure true) 0.05))
            (:`2`
              (goto _label_5))
            (:`3`
              (goto _label_6))
            (:`4`
              (goto _label_6))
            (:`5`
              (`/Game/MyStuff/UI/WID_PlayerHud.RefusedBag` (`self.playerHud`)))))
        (:`4`
          (goto _label_4))
        (:`5`
          (goto _label_4))))))

(fn `UserConstructionScript`)